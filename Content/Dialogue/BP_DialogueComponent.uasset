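; BP_DialogueComponent is a dialogue component that runs branching, data-table-driven conversations in a UI widget.
; Interact creates WB_Dialogue with the cursor shown, advances through linked rows, and closes it once EndDialogue is set.
; The opening row, if open-ended, and every selected option's row spawn WB_OptionsDialogue choices carrying their target row and table.
; LeaveDialogue removes the widget and restores game-only input.
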(event Custom|Option%20Selected
  (params (RowName :type Name) (DataTable :type Data%20Table%20Object%20Reference))
  (bind _dialoguewidget (Variables|Default|GetDialogueWidget))
  ;[0.05098 0.05098 0.05098] Options Selection
  (bind _returnvalue (Utilities|GetDataTableRow DataTable RowName)
    (:then
      (Widget|Panel|ClearChildren (Variables|/Game/Dialogue/WB_Dialogue.WB_Dialogue_C|GetOptionsScrollBox _dialoguewidget))
      (Default|UpdateDialogue _dialoguewidget (.Dialogue (Utilities|Struct|BreakDialogue_Structure _returnvalue)))
      (Variables|Default|SetRow%20Name (.Row (Utilities|Struct|BreakDialogue_Structure _returnvalue)))
      (Variables|Default|SetData%20Table (.DataTable (Utilities|Struct|BreakDialogue_Structure _returnvalue)))
      (Variables|Default|SetEndDialogue (.EndDialogue? (Utilities|Struct|BreakDialogue_Structure _returnvalue)))
      ;[0.05098 0.05098 0.05098] Showing even more Options
      (if true
        (for _array_element (.OpenEndedDialogueOptions (Utilities|Struct|BreakDialogue_Structure _returnvalue))
          (bind _returnvalue_2 (UserInterface|CreateWidget "/Game/Dialogue/WB_OptionsDialogue.WB_OptionsDialogue_C" 0 (Utilities|Text|ToText(Name) (.Optionname (Utilities|Struct|BreakOptionsDialogue_Structure _array_element))) self (.Row (Utilities|Struct|BreakOptionsDialogue_Structure _array_element)) (.Datatable (Utilities|Struct|BreakOptionsDialogue_Structure _array_element))))
          (Widget|Panel|AddChild (Variables|/Game/Dialogue/WB_Dialogue.WB_Dialogue_C|GetOptionsScrollBox (Variables|Default|GetDialogueWidget)) _returnvalue_2))))))

(event EventBeginPlay)

(event EventTick
  (params (DeltaSeconds :type Float%20%28single-precision%29)))

(event EventInteract
  (params (playerref :type BP%20First%20Person%20Character%20Object%20Reference))
  (bind _returnvalue (Game|GetPlayerController 0))
  (bind _returnvalue_2 (Game|GetPlayerController 0))
  ;[0.05098 0.05098 0.05098] Making NPC's Interactable
  (if (Variables|Default|GetEndDialogue)
    (Widget|RemovefromParent (Variables|Default|GetDialogueWidget))
    (Variables|Default|SetEndDialogue false)
    (Variables|Default|SetDialogueWidget 0)
    ;[0.05098 0.05098 0.05098] Hide Mouse Cursor
    (Input|SetInputModeGameOnly _returnvalue_2 false)
    (Variables|/Script/Engine.PlayerController|SetbShowMouseCursor _returnvalue_2 false)
    (else
      (Utilities|IsValid (Variables|Default|GetDialogueWidget)
        (:Is%20Valid
          ;[0.05098 0.05098 0.05098] Allowing longer dialogue trees
          (bind _returnvalue_3 (Utilities|GetDataTableRow (Variables|Default|GetData%20Table) (Variables|Default|GetRow%20Name))
            (:then
              (Default|UpdateDialogue (Variables|Default|GetDialogueWidget) (.Dialogue (Utilities|Struct|BreakDialogue_Structure _returnvalue_3)))
              (Variables|Default|SetRow%20Name (.Row (Utilities|Struct|BreakDialogue_Structure _returnvalue_3)))
              (Variables|Default|SetData%20Table (.DataTable (Utilities|Struct|BreakDialogue_Structure _returnvalue_3)))
              (Variables|Default|SetEndDialogue (.EndDialogue? (Utilities|Struct|BreakDialogue_Structure _returnvalue_3))))))
        (:Is%20Not%20Valid
          ;[0.05098 0.05098 0.05098] Showing Dialogue
          (Development|PrintString "Interaction success")
          (bind _returnvalue_4 (Utilities|GetDataTableRow (Variables|Default|GetData%20Table) (Variables|Default|GetRow%20Name))
            (:then
              (bind _returnvalue_5 (UserInterface|CreateWidget "/Game/Dialogue/WB_Dialogue.WB_Dialogue_C" 0 (Utilities|Text|ToText(Name) (Variables|Default|GetName)) (.Dialogue (Utilities|Struct|BreakDialogue_Structure _returnvalue_4))))
              (bind _output_get (Variables|Default|SetDialogueWidget _returnvalue_5))
              (UserInterface|Viewport|AddtoViewport _output_get 0)
              (Variables|Default|SetRow%20Name (.Row (Utilities|Struct|BreakDialogue_Structure _returnvalue_4)))
              (Variables|Default|SetData%20Table (.DataTable (Utilities|Struct|BreakDialogue_Structure _returnvalue_4)))
              (Variables|Default|SetEndDialogue (.EndDialogue? (Utilities|Struct|BreakDialogue_Structure _returnvalue_4)))
              ;[0.05098 0.05098 0.05098] Show Mouse
              (Input|SetInputModeGameandUI _returnvalue 0 "DoNotLock" true false)
              (Variables|/Script/Engine.PlayerController|SetbShowMouseCursor _returnvalue true)
              (if (.Openendeddialogue? (Utilities|Struct|BreakDialogue_Structure _returnvalue_4))
                ;[0.05098 0.05098 0.05098] Options can be chosen
                (for _array_element (.OpenEndedDialogueOptions (Utilities|Struct|BreakDialogue_Structure _returnvalue_4))
                  (bind _returnvalue_6 (UserInterface|CreateWidget "/Game/Dialogue/WB_OptionsDialogue.WB_OptionsDialogue_C" 0 (Utilities|Text|ToText(Name) (.Optionname (Utilities|Struct|BreakOptionsDialogue_Structure _array_element))) self (.Row (Utilities|Struct|BreakOptionsDialogue_Structure _array_element)) (.Datatable (Utilities|Struct|BreakOptionsDialogue_Structure _array_element))))
                  (Widget|Panel|AddChild (Variables|/Game/Dialogue/WB_Dialogue.WB_Dialogue_C|GetOptionsScrollBox (Variables|Default|GetDialogueWidget)) _returnvalue_6))))))))))

(event EventLeaveDialogue
  (bind _returnvalue (Game|GetPlayerController 0))
  ;[0.05098 0.05098 0.05098] Make dialogue leavable
  (Utilities|IsValid (Variables|Default|GetDialogueWidget)
    (:Is%20Valid
      ;[0.05098 0.05098 0.05098] Making NPC's Interactable
      (Widget|RemovefromParent (Variables|Default|GetDialogueWidget))
      (Variables|Default|SetEndDialogue false)
      (Variables|Default|SetDialogueWidget 0)
      ;[0.05098 0.05098 0.05098] Hide Mouse Cursor
      (Input|SetInputModeGameOnly _returnvalue false)
      (Variables|/Script/Engine.PlayerController|SetbShowMouseCursor _returnvalue false))))